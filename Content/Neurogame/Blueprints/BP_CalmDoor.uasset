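; Door actor that rises with the player's calm score from the Neurosity interface.
; BeginPlay caches the player and door start position, adds the input mapping, and retries until it finds the interface actor.
; Each Tick rebuilds a blue glow material driven by the focus score, not calm.
; With the player nearby and relax power on, calm lifts the door within a height limit; otherwise it eases back to its start.
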(event `self.ReceiveBeginPlay`
  (bind _returnvalue (pcsubsystem `EnhancedInputLocalPlayerSubsystem` (`GameplayStatics.GetPlayerController` 0)))
  ;[1 1 1] Get the Enhanced Input Controlle System. We're gonna need it.
  (bind _asbp_third_person_character_neurogame (cast `/Game/ThirdPerson/Blueprints/BP_ThirdPersonCharacter_Neurogame` (`GameplayStatics.GetPlayerCharacter` 0)))
  (set `self.The Player Character` _asbp_third_person_character_neurogame)
  (`/Engine/EditorBlueprintResources/StandardMacros.IsValid` _returnvalue
    (:`Is Valid`
      (`EnhancedInputSubsystemInterface.AddMappingContext` _returnvalue "/Game/ThirdPerson/Input/IMC_Default.IMC_Default" 0 (struct))
      ;[1 1 1] We're going to make this door float. Since I don't want it to move upwards indefinitely, I want to make sure where we start.
      (set `self.My Initial Position` (`SceneComponent.RelativeLocation` (`self.Door`)))
      ;[1 1 1] Here we try to fish for the Neurosity Interface instance. We delay further action until we're certain we got it. Sometimes instancing can take a bit, so here's a couple failsafes.
      (bind _returnvalue_2 (`GameplayStatics.GetActorOfClass` "/Game/Neurogame/Blueprints/BP_NeurosityInterface.BP_NeurosityInterface_C" :!label _label))
      (bind _asbp_neurosity_interface (cast `/Game/Neurogame/Blueprints/BP_NeurosityInterface` _returnvalue_2)
        (:`then`
          (set `self.Level Neurosity Interface` _asbp_neurosity_interface)
          (`/Engine/EditorBlueprintResources/StandardMacros.IsValid` (`self.Level Neurosity Interface`)
            (:`Is Not Valid`
              _)))
        (:`CastFailed`
          _))
      (`KismetSystemLibrary.Delay` 0.2)
      (goto _label))))

(event `self.ReceiveTick`
  (params (DeltaSeconds :type "Float (single-precision)"))
  (bind (_x _y _z) (`KismetMathLibrary.BreakVector3f` (`self.My Initial Position`)))
  (bind _focusscoreprobability (`/Game/Neurogame/Blueprints/BP_NeurosityInterface.FocusScoreProbability` (`self.Level Neurosity Interface`)))
  ;[1 1 1] Failsafe. Only proceed if the Neurosity Interface has been caught. See failsafes above.
  (`/Engine/EditorBlueprintResources/StandardMacros.IsValid` (`self.Level Neurosity Interface`)
    (:`Is Valid`
      ;[1 1 1] Here, we color the cube according to how focused you are. From the Dynamic Material instance, we start with a minimum emission of 50 and keep adding as the probability goes up. The multiplication is there because we're given decimals as our focus score.
      ;
      ; Same goes for Color. We start with a Green value of 0.5 and go up as Focus goes up. Since I don't want the color valie to go beyond 1, I divide the score by two, since we already have half the green covered as our baseline..
      (bind _returnvalue (`PrimitiveComponent.CreateDynamicMaterialInstance` (`self.Glow1`) 0 "/Game/Neurogame/Materials/Material_CalmGlowBlue.Material_CalmGlowBlue" "None"))
      (`MaterialInstanceDynamic.SetScalarParameterValue` _returnvalue "Emission" (+ (* _focusscoreprobability 10.0) 5.0))
      (`MaterialInstanceDynamic.SetVectorParameterValue` _returnvalue "Color" (make `LinearColor` 0.0 0.3 (+ (/ _focusscoreprobability 2.0) 0.5) 1.0))
      (`PrimitiveComponent.SetMaterial` (`self.Glow1`) 0 _returnvalue)
      (`PrimitiveComponent.SetMaterial` (`self.Glow2`) 0 _returnvalue)
      ;[1 1 1] Let's make certain that the player is close enough to be relevant. Three meters seems about right.
      (if (< (`self.GetDistanceTo` (`GameplayStatics.GetPlayerCharacter` 0) self) 300.0)
        ;[1 1 1] If the neuro power is on (press X), raise the platform. Otherwise, put it back to its initial state.
        (bind _asbp_neuro_player_controller (cast `/Game/Blueprints/BP_NeuroPlayerController` (`Pawn.GetController` (`self.The Player Character`))))
        (if (`/Game/Blueprints/BP_NeuroPlayerController.isRelaxOn` _asbp_neuro_player_controller)
          ;[1 1 1] Let's limit the door's flight height to 1 meter up.
          (if (< (`.Z` (`KismetMathLibrary.BreakVector3f` (`SceneComponent.RelativeLocation` (`self.Door`)))) 300.0)
            ;[1 1 1] Smoothly move the door upwards in relation to the initial position. The multiplication is there to make movement significantly noticeable, since we're fed a Calm score in decimals.
            (`KismetSystemLibrary.MoveComponentTo` (`self.Door`) (+ (`self.My Initial Position`) (`KismetMathLibrary.MakeVector` 0.0 0.0 (* (`/Game/Neurogame/Blueprints/BP_NeurosityInterface.CalmScoreProbability` (`self.Level Neurosity Interface`)) (`self.Relax Multiplier`)))) (struct) true true)
            (else
              ;[1 1 1] Otherwise, move the door back down to its original position.
              (`SceneComponent.K2_SetRelativeLocation` (`self.Door`) (`KismetMathLibrary.MakeVector` _x _y (+ _z 200.0)) false false)))
          (else
            (`KismetSystemLibrary.MoveComponentTo` (`self.Door`) (`self.My Initial Position`) (struct) true true 0.25 :!label _label_2)))
        (else
          (goto _label_2))))))

(fn `UserConstructionScript`)